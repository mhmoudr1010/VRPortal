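; BP_RightTriggerBox is a trigger in the DataPrivacy level that records which personal and non-personal data boxes enter it.
; Overlaps add each box's text-type enum to a unique string list and print the list.
; A six-second looping timer copies the list to the GameInstance and calls SendBoxScores.
; A one-time Tick bind to the spawner's game-finished event triggers a delayed Firebase score upload through the GameInstance.
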(event `self.ReceiveBeginPlay`
  (bind _asportal_game_instance (cast `PortalGameInstance` (`GameplayStatics.GetGameInstance`)))
  (set `self.GameInstance` _asportal_game_instance)
  (bind _returnvalue (`GameplayStatics.GetActorOfClass` "/Game/Level_Content/DataPrivacy/Blueprints/Spawner/BP_Spawner.BP_Spawner_C"))
  (set `self.Spawner` _returnvalue)
  (`KismetSystemLibrary.K2_SetTimer` null "SaveBoxesWithScore" 6.0 true))

(event `self.ReceiveActorBeginOverlap`
  (params (OtherActor :type "Actor Object Reference"))
  (`|ExecutionSequence`
    (:`then_0`
      (bind _asbp_personal_data_box (cast `/Game/Level_Content/DataPrivacy/Blueprints/BP_PersonalDataBox` OtherActor))
      (`KismetArrayLibrary.Array_AddUnique` (`self.Boxes`) (`|GetEnumeratorNameAsString` (`/Game/Level_Content/DataPrivacy/Blueprints/BP_PersonalDataBox.ENumTextType` _asbp_personal_data_box)))
      (for _array_element (`self.Boxes`)
        (`KismetSystemLibrary.PrintString` _array_element)))
    (:`then_1`
      (bind _asbp_non_personal_data_box (cast `/Game/Level_Content/DataPrivacy/Blueprints/BP_NonPersonalDataBox` OtherActor))
      (`KismetArrayLibrary.Array_AddUnique` (`self.Boxes`) (`|GetEnumeratorNameAsString` (`/Game/Level_Content/DataPrivacy/Blueprints/BP_NonPersonalDataBox.ENumTextType` _asbp_non_personal_data_box)))
      (for _array_element_2 (`self.Boxes`)
        (`KismetSystemLibrary.PrintString` _array_element_2)))))

(event `self.ReceiveTick`
  (params (DeltaSeconds :type "Float (single-precision)"))
  (`/Engine/EditorBlueprintResources/StandardMacros.DoOnce` false
    (:`Completed`
      (add `/Game/Level_Content/DataPrivacy/Blueprints/Spawner/BP_Spawner.OnGameFinished` (`self.Spawner`) (delegate `OnGameFinished_Event`)))))

(event `OnGameFinished_Event`
  (`KismetSystemLibrary.PrintString` "Sending BoxesScore")
  (`KismetSystemLibrary.Delay` 5.0)
  (`PortalGameInstance.SendBoxScoresToFirebase1` (`self.GameInstance`)))

(fn `SaveBoxesWithScore`
  (bind _gameinstance (`self.GameInstance`))
  (set `PortalGameInstance.ClaimedBoxes` (`self.Boxes`) _gameinstance)
  (`PortalGameInstance.SendBoxScores` _gameinstance))

(fn `UserConstructionScript`)