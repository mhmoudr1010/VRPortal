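; Physics-driven VR or grabbable box for a data privacy level, showing an Arabic personal-data label on six face widgets, chosen by ENumTextType.
; Unless held, finished or static, Tick pushes it toward BP_EndCube with random chaos force and binds the grab event.
; Grabbing stops the push, restores gravity and enables simulate-on-drop.
; TriggerTextOnNameBP can set BP_Name's explanation text but is unused here; spline movement is dead code.
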(event `self.ReceiveBeginPlay`
  (set `self.CurrentDistance` 0.0)
  (set `self.IsHeld` false)
  (set `self.InitialTransform` (`self.GetTransform`))
  (bind _returnvalue (`GameplayStatics.GetActorOfClass` "/Game/Level_Content/DataPrivacy/Blueprints/BP_EndCube.BP_EndCube_C"))
  (set `self.EndCube` _returnvalue)
  (`KismetSystemLibrary.Delay` 1.0)
  (`self.SetNameOnBox` (`self.WidgetForward`))
  (`self.SetNameOnBox` (`self.WidgetTop`))
  (`self.SetNameOnBox` (`self.WidgetBottom`))
  (`self.SetNameOnBox` (`self.WidgetRight`))
  (`self.SetNameOnBox` (`self.WidgetLeft`))
  (`self.SetNameOnBox` (`self.WidgetBack`)))

(event `self.ReceiveTick`
  (params (DeltaSeconds :type "Float (single-precision)"))
  (if (not (or (`self.IsHeld`) (`self.IsFinished`) (`self.IsStatic`)))
    (`PrimitiveComponent.AddForce` (`self.StaticMesh`) (* (`KismetMathLibrary.VLerp` (`KismetMathLibrary.Normal` (- (`self.K2_GetActorLocation` (`self.EndCube`)) (`self.K2_GetActorLocation`))) (* (`KismetMathLibrary.MakeVector` (`KismetMathLibrary.RandomFloatInRange` -1.0 1.0) (`KismetMathLibrary.RandomFloatInRange` -1.0 1.0) (`KismetMathLibrary.RandomFloatInRange` -1.0 1.0)) (`self.ChaosStrength`)) 0.7) (`self.ForceStrength`)) "None" false)
    ;[1 1 1] Enable Physics again after being grabbed
    (add `/Game/VRTemplate/Blueprints/GrabComponent.OnGrabbed` (`self.GrabComponent`) (delegate `OnGrabbed_Event`))))

(event `OnGrabbed_Event`
  ;[1 1 1] Enable Physics again after being grabbed
  (`self.HandleAfterGrabbed`))

(fn `HandleAfterGrabbed`
  (set `self.IsHeld` true)
  (set `/Game/VRTemplate/Blueprints/GrabComponent.bSimulateOnDrop` true (`self.GrabComponent`))
  (`PrimitiveComponent.SetEnableGravity` (`self.StaticMesh`) true))

(fn `SetNameOnBox`
  (params (self2 :type "WidgetComponent Object Reference"))
  (bind _aswbp_name_on_box (cast `/Game/Level_Content/DataPrivacy/Blueprints/Widgets/WBP_NameOnBox` (`WidgetComponent.GetWidget` self2)))
  (switch `/Game/Level_Content/DataPrivacy/Blueprints/E_TextType` (`self.ENumTextType`)
    (:`NewEnumerator0`
      (set `/Game/Level_Content/DataPrivacy/Blueprints/Widgets/WBP_NameOnBox.NameOnBox` "اسم الشخص" _aswbp_name_on_box))
    (:`NewEnumerator1`
      (set `/Game/Level_Content/DataPrivacy/Blueprints/Widgets/WBP_NameOnBox.NameOnBox` "العنوان الشخصي" _aswbp_name_on_box))
    (:`NewEnumerator2`
      (set `/Game/Level_Content/DataPrivacy/Blueprints/Widgets/WBP_NameOnBox.NameOnBox` "رقم الحساب البنكي" _aswbp_name_on_box))
    (:`NewEnumerator3`
      (set `/Game/Level_Content/DataPrivacy/Blueprints/Widgets/WBP_NameOnBox.NameOnBox` "تاريخ الميلاد" _aswbp_name_on_box))
    (:`NewEnumerator4`
      (set `/Game/Level_Content/DataPrivacy/Blueprints/Widgets/WBP_NameOnBox.NameOnBox` "الايميل الشخصي" _aswbp_name_on_box))))

(fn `TriggerTextOnNameBP`
  (bind _outactors (`GameplayStatics.GetAllActorsOfClass` "/Game/Level_Content/DataPrivacy/Blueprints/BP_Name.BP_Name_C"))
  (bind _aswbp_name (cast `/Game/Level_Content/DataPrivacy/Blueprints/Widgets/WBP_Name` (`WidgetComponent.GetWidget` (`/Game/Level_Content/DataPrivacy/Blueprints/BP_Name.TextWidget` (`|GetArrayItem` _outactors)))))
  (switch `/Game/Level_Content/DataPrivacy/Blueprints/E_TextType` (`self.ENumTextType`)
    (:`NewEnumerator0`
      (set `/Game/Level_Content/DataPrivacy/Blueprints/Widgets/WBP_Name.Text` "اسم الشخص: \nلأنه معرّف فريد ويرتبط بهوية الشخص." _aswbp_name))
    (:`NewEnumerator1`
      (set `/Game/Level_Content/DataPrivacy/Blueprints/Widgets/WBP_Name.Text` "العنوان الشخصي: \nلأنه يكشف عن مكان إقامة الشخص \n ويمكن استخدامه لتحديد هويته." _aswbp_name))
    (:`NewEnumerator2`
      (set `/Game/Level_Content/DataPrivacy/Blueprints/Widgets/WBP_Name.Text` "رقم الحساب البنكي: \nلأنه مرتبط بمعلومات مالية حساسة \n خاصة بـ صاحب الحساب." _aswbp_name))
    (:`NewEnumerator3`
      (set `/Game/Level_Content/DataPrivacy/Blueprints/Widgets/WBP_Name.Text` "تاريخ الميلاد: \nلأنه معرّف فريد ويساعد في تحديد  \nهوية الشخص." _aswbp_name))
    (:`NewEnumerator4`
      (set `/Game/Level_Content/DataPrivacy/Blueprints/Widgets/WBP_Name.Text` "الايميل الشخصي: \nلأنه يستخدم للتواصل مع صاحب البريد \n ويمكن أن يحتوي على  \nمعلومات شخصية." _aswbp_name))))

(fn `UserConstructionScript`)