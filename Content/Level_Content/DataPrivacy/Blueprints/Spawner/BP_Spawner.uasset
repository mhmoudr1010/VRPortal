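; Data privacy level spawner that drops personal and non-personal data boxes at random points in its box volume and tracks level duration.
; After a delay, a timer spawns classes from an ordered array and assigns each box a fixed text type by index.
; Once nine exist, Tick binds the last box's overlap to end the game.
; That broadcasts game finished, enables the finish trigger, reveals static boxes and score, and plays end audio.
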(event `self.ReceiveBeginPlay`
  ;[1 1 1] Timer to save Level Duration
  (bind _returnvalue (`KismetSystemLibrary.K2_SetTimer` null "UpdateTimer" 1.0 true))
  (set `self.TimerHandle` _returnvalue)
  (`KismetSystemLibrary.Delay` 13.0)
  (`KismetSystemLibrary.K2_SetTimerDelegate` (delegate `SpawnDataBox`) (`self.SpawnTime`) (`self.Looping`)))

(event `SpawnDataBox`
  (bind _spawneddataboxes (`self.SpawnedDataBoxes`))
  (bind _result (`/Engine/EditorBlueprintResources/StandardMacros.IncrementInt` (`self.LoopCounter`))
    (:`  `
      (if (< _result 10)
        (bind _returnvalue (`|SpawnActorFromClass` (`|GetArrayItem` (`self.DataBoxClass`) (`self.CurrentIndex`)) (`KismetMathLibrary.MakeTransform` (`self.GetRandomPointInBoxExtend`) (`KismetMathLibrary.RandomRotator` false)) "AlwaysSpawn" "MultiplyWithRoot" null null))
        (`/Engine/EditorBlueprintResources/StandardMacros.IncrementInt` (`self.CurrentIndex`)
          (:`  `
            (`KismetArrayLibrary.Array_Add` _spawneddataboxes _returnvalue)
            (`|ExecutionSequence`
              (:`then_0`
                (bind _asbp_personal_data_box (cast `/Game/Level_Content/DataPrivacy/Blueprints/BP_PersonalDataBox` (`|GetArrayItem` _spawneddataboxes)))
                (set `/Game/Level_Content/DataPrivacy/Blueprints/BP_PersonalDataBox.ENumTextType` "NewEnumerator0" _asbp_personal_data_box))
              (:`then_1`
                (bind _asbp_non_personal_data_box (cast `/Game/Level_Content/DataPrivacy/Blueprints/BP_NonPersonalDataBox` (`|GetArrayItem` _spawneddataboxes 1)))
                (set `/Game/Level_Content/DataPrivacy/Blueprints/BP_NonPersonalDataBox.ENumTextType` "NewEnumerator5" _asbp_non_personal_data_box))
              (:`then_2`
                (bind _asbp_non_personal_data_box_2 (cast `/Game/Level_Content/DataPrivacy/Blueprints/BP_NonPersonalDataBox` (`|GetArrayItem` _spawneddataboxes 2)))
                (set `/Game/Level_Content/DataPrivacy/Blueprints/BP_NonPersonalDataBox.ENumTextType` "NewEnumerator6" _asbp_non_personal_data_box_2))
              (:`then_3`
                (bind _asbp_personal_data_box_2 (cast `/Game/Level_Content/DataPrivacy/Blueprints/BP_PersonalDataBox` (`|GetArrayItem` _spawneddataboxes 3)))
                (set `/Game/Level_Content/DataPrivacy/Blueprints/BP_PersonalDataBox.ENumTextType` "NewEnumerator1" _asbp_personal_data_box_2))
              (:`then_4`
                (bind _asbp_non_personal_data_box_3 (cast `/Game/Level_Content/DataPrivacy/Blueprints/BP_NonPersonalDataBox` (`|GetArrayItem` _spawneddataboxes 4)))
                (set `/Game/Level_Content/DataPrivacy/Blueprints/BP_NonPersonalDataBox.ENumTextType` "NewEnumerator7" _asbp_non_personal_data_box_3))
              (:`then_5`
                (bind _asbp_personal_data_box_3 (cast `/Game/Level_Content/DataPrivacy/Blueprints/BP_PersonalDataBox` (`|GetArrayItem` _spawneddataboxes 5)))
                (set `/Game/Level_Content/DataPrivacy/Blueprints/BP_PersonalDataBox.ENumTextType` "NewEnumerator2" _asbp_personal_data_box_3))
              (:`then_6`
                (bind _asbp_personal_data_box_4 (cast `/Game/Level_Content/DataPrivacy/Blueprints/BP_PersonalDataBox` (`|GetArrayItem` _spawneddataboxes 6)))
                (set `/Game/Level_Content/DataPrivacy/Blueprints/BP_PersonalDataBox.ENumTextType` "NewEnumerator3" _asbp_personal_data_box_4))
              (:`then_7`
                (bind _asbp_non_personal_data_box_4 (cast `/Game/Level_Content/DataPrivacy/Blueprints/BP_NonPersonalDataBox` (`|GetArrayItem` _spawneddataboxes 7)))
                (set `/Game/Level_Content/DataPrivacy/Blueprints/BP_NonPersonalDataBox.ENumTextType` "NewEnumerator8" _asbp_non_personal_data_box_4))
              (:`then_8`
                (bind _asbp_personal_data_box_5 (cast `/Game/Level_Content/DataPrivacy/Blueprints/BP_PersonalDataBox` (`|GetArrayItem` _spawneddataboxes 8)))
                (set `/Game/Level_Content/DataPrivacy/Blueprints/BP_PersonalDataBox.ENumTextType` "NewEnumerator4" _asbp_personal_data_box_5)))))
        (else
          (set `self.Looping` false))))))

(event `self.ReceiveTick`
  (params (DeltaSeconds :type "Float (single-precision)"))
  (bind _spawneddataboxes (`self.SpawnedDataBoxes`))
  (if (== (`KismetArrayLibrary.Array_Length` _spawneddataboxes) 9)
    (bind _asbp_personal_data_box (cast `/Game/Level_Content/DataPrivacy/Blueprints/BP_PersonalDataBox` (`|GetArrayItem` _spawneddataboxes 8))
      (:`then`
        (add `self.OnActorBeginOverlap` _asbp_personal_data_box (delegate `OnActorBeginOverlap_Event`)))
      (:`CastFailed`
        (`KismetSystemLibrary.PrintString` "Failed to Cast from Spawner")))))

(event `OnActorBeginOverlap_Event` :!signature `self.OnActorBeginOverlap`
  (params (OverlappedActor :type "Actor Object Reference") (OtherActor :type "Actor Object Reference"))
  (`|ExecutionSequence`
    (:`then_0`
      (`self.OnGameFinished`)
      (bind _returnvalue (`GameplayStatics.GetActorOfClass` "/Game/Level_Content/DataPrivacy/Blueprints/BP_FinishTriggerBox.BP_FinishTriggerBox_C"))
      (`PrimitiveComponent.SetCollisionEnabled` (`/Game/Level_Content/DataPrivacy/Blueprints/BP_FinishTriggerBox.Box` _returnvalue) "QueryAndPhysics")
      (for _array_element (`/Game/Level_Content/DataPrivacy/Blueprints/BP_FinishTriggerBox.StaticDataBoxes` _returnvalue)
        (`self.SetActorHiddenInGame` _array_element false)
        (bind _returnvalue_2 (`GameplayStatics.GetActorOfClass` "/Game/Level_Content/DataPrivacy/Blueprints/BP_Name.BP_Name_C"))
        (`SceneComponent.SetVisibility` (`/Game/Level_Content/DataPrivacy/Blueprints/BP_Name.ScoreWidget` _returnvalue_2) true false)
        (`KismetSystemLibrary.Delay` 5.0)
        (`GameplayStatics.PlaySound2D` "/Game/Level_Content/DataPrivacy/Assets/Sounds/GameEnd.GameEnd" 1.0 1.0 0.0 null null))
      (`KismetSystemLibrary.PrintString` "All Static boxes are visibile again "))))

(fn `GetRandomPointInBoxExtend`
  (returns (ReturnValue :type "Vector Structure"))
  (bind (_returnvalue_x _returnvalue_y _returnvalue_z) (`KismetMathLibrary.BreakVector` (`BoxComponent.GetScaledBoxExtent` (`self.Box`))))
  (return (+ (`SceneComponent.K2_GetComponentLocation` (`self.Box`)) (`KismetMathLibrary.MakeVector` (`KismetMathLibrary.RandomFloatInRange` (* _returnvalue_x -1.0) _returnvalue_x) (`KismetMathLibrary.RandomFloatInRange` (* _returnvalue_y -1.0) _returnvalue_y) (`KismetMathLibrary.RandomFloatInRange` (* _returnvalue_z -1.0) _returnvalue_z)))))

(fn `UpdateTimer`
  (`/Engine/EditorBlueprintResources/StandardMacros.IncrementFloat` (`self.LevelDuration`)))

(fn `UserConstructionScript`)