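; Finish trigger for the data privacy level that catches personal and non-personal data boxes.
; On overlap it triggers the box's name text, plays a bubble sound, releases the grab, ignores PhysicsBody collision and teleports the box to its initial transform.
; BeginPlay collects and hides actors tagged StaticDataBox.
; Tick re-binds their grab events every frame by fixed array index, so grabbing marks them held and restores gravity and drop physics.
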(event `CustomEvent_7`
  ;[1 1 1] Enable Physics again after being grabbed
  (set `/Game/Level_Content/DataPrivacy/Blueprints/BP_NonPersonalDataBox.IsHeld` true (stale `self.ReceiveTick` _asbp_non_personal_data_box))
  (set `/Game/VRTemplate/Blueprints/GrabComponent.bSimulateOnDrop` true (`/Game/Level_Content/DataPrivacy/Blueprints/BP_NonPersonalDataBox.GrabComponent` (stale `self.ReceiveTick` _asbp_non_personal_data_box)))
  (`PrimitiveComponent.SetEnableGravity` (`/Game/Level_Content/DataPrivacy/Blueprints/BP_NonPersonalDataBox.StaticMesh` (stale `self.ReceiveTick` _asbp_non_personal_data_box)) true))

(event `CustomEvent_6`
  ;[1 1 1] Enable Physics again after being grabbed
  (set `/Game/Level_Content/DataPrivacy/Blueprints/BP_NonPersonalDataBox.IsHeld` true (stale `self.ReceiveTick` _asbp_non_personal_data_box_2))
  (set `/Game/VRTemplate/Blueprints/GrabComponent.bSimulateOnDrop` true (`/Game/Level_Content/DataPrivacy/Blueprints/BP_NonPersonalDataBox.GrabComponent` (stale `self.ReceiveTick` _asbp_non_personal_data_box_2)))
  (`PrimitiveComponent.SetEnableGravity` (`/Game/Level_Content/DataPrivacy/Blueprints/BP_NonPersonalDataBox.StaticMesh` (stale `self.ReceiveTick` _asbp_non_personal_data_box_2)) true))

(event `CustomEvent_5`
  ;[1 1 1] Enable Physics again after being grabbed
  (set `/Game/Level_Content/DataPrivacy/Blueprints/BP_NonPersonalDataBox.IsHeld` true (stale `self.ReceiveTick` _asbp_non_personal_data_box_3))
  (set `/Game/VRTemplate/Blueprints/GrabComponent.bSimulateOnDrop` true (`/Game/Level_Content/DataPrivacy/Blueprints/BP_NonPersonalDataBox.GrabComponent` (stale `self.ReceiveTick` _asbp_non_personal_data_box_3)))
  (`PrimitiveComponent.SetEnableGravity` (`/Game/Level_Content/DataPrivacy/Blueprints/BP_NonPersonalDataBox.StaticMesh` (stale `self.ReceiveTick` _asbp_non_personal_data_box_3)) true))

(event `CustomEvent_4`
  ;[1 1 1] Enable Physics again after being grabbed
  (set `/Game/Level_Content/DataPrivacy/Blueprints/BP_NonPersonalDataBox.IsHeld` true (stale `self.ReceiveTick` _asbp_non_personal_data_box_4))
  (set `/Game/VRTemplate/Blueprints/GrabComponent.bSimulateOnDrop` true (`/Game/Level_Content/DataPrivacy/Blueprints/BP_NonPersonalDataBox.GrabComponent` (stale `self.ReceiveTick` _asbp_non_personal_data_box_4)))
  (`PrimitiveComponent.SetEnableGravity` (`/Game/Level_Content/DataPrivacy/Blueprints/BP_NonPersonalDataBox.StaticMesh` (stale `self.ReceiveTick` _asbp_non_personal_data_box_4)) true))

(event `self.ReceiveTick`
  (params (DeltaSeconds :type "Float (single-precision)"))
  (`|ExecutionSequence`
    (:`then_0`
      (bind _asbp_non_personal_data_box (cast `/Game/Level_Content/DataPrivacy/Blueprints/BP_NonPersonalDataBox` (`|GetArrayItem` (`self.StaticDataBoxes`))))
      ;[1 1 1] Enable Physics again after being grabbed
      (add `/Game/VRTemplate/Blueprints/GrabComponent.OnGrabbed` (`/Game/Level_Content/DataPrivacy/Blueprints/BP_NonPersonalDataBox.GrabComponent` _asbp_non_personal_data_box) (delegate `CustomEvent_7`)))
    (:`then_1`
      (bind _asbp_non_personal_data_box_2 (cast `/Game/Level_Content/DataPrivacy/Blueprints/BP_NonPersonalDataBox` (`|GetArrayItem` (`self.StaticDataBoxes`) 1)))
      ;[1 1 1] Enable Physics again after being grabbed
      (add `/Game/VRTemplate/Blueprints/GrabComponent.OnGrabbed` (`/Game/Level_Content/DataPrivacy/Blueprints/BP_NonPersonalDataBox.GrabComponent` _asbp_non_personal_data_box_2) (delegate `CustomEvent_6`)))
    (:`then_2`
      (bind _asbp_non_personal_data_box_3 (cast `/Game/Level_Content/DataPrivacy/Blueprints/BP_NonPersonalDataBox` (`|GetArrayItem` (`self.StaticDataBoxes`) 2)))
      ;[1 1 1] Enable Physics again after being grabbed
      (add `/Game/VRTemplate/Blueprints/GrabComponent.OnGrabbed` (`/Game/Level_Content/DataPrivacy/Blueprints/BP_NonPersonalDataBox.GrabComponent` _asbp_non_personal_data_box_3) (delegate `CustomEvent_5`)))
    (:`then_3`
      (bind _asbp_non_personal_data_box_4 (cast `/Game/Level_Content/DataPrivacy/Blueprints/BP_NonPersonalDataBox` (`|GetArrayItem` (`self.StaticDataBoxes`) 3)))
      ;[1 1 1] Enable Physics again after being grabbed
      (add `/Game/VRTemplate/Blueprints/GrabComponent.OnGrabbed` (`/Game/Level_Content/DataPrivacy/Blueprints/BP_NonPersonalDataBox.GrabComponent` _asbp_non_personal_data_box_4) (delegate `CustomEvent_4`)))
    (:`then_4`
      (bind _asbp_personal_data_box (cast `/Game/Level_Content/DataPrivacy/Blueprints/BP_PersonalDataBox` (`|GetArrayItem` (`self.StaticDataBoxes`) 4)))
      ;[1 1 1] Enable Physics again after being grabbed
      (add `/Game/VRTemplate/Blueprints/GrabComponent.OnGrabbed` (`/Game/Level_Content/DataPrivacy/Blueprints/BP_PersonalDataBox.GrabComponent` _asbp_personal_data_box) (delegate `OnGrabbed_Event`)))
    (:`then_5`
      (bind _asbp_personal_data_box_2 (cast `/Game/Level_Content/DataPrivacy/Blueprints/BP_PersonalDataBox` (`|GetArrayItem` (`self.StaticDataBoxes`) 5)))
      ;[1 1 1] Enable Physics again after being grabbed
      (add `/Game/VRTemplate/Blueprints/GrabComponent.OnGrabbed` (`/Game/Level_Content/DataPrivacy/Blueprints/BP_PersonalDataBox.GrabComponent` _asbp_personal_data_box_2) (delegate `CustomEvent`)))
    (:`then_6`
      (bind _asbp_personal_data_box_3 (cast `/Game/Level_Content/DataPrivacy/Blueprints/BP_PersonalDataBox` (`|GetArrayItem` (`self.StaticDataBoxes`) 6)))
      ;[1 1 1] Enable Physics again after being grabbed
      (add `/Game/VRTemplate/Blueprints/GrabComponent.OnGrabbed` (`/Game/Level_Content/DataPrivacy/Blueprints/BP_PersonalDataBox.GrabComponent` _asbp_personal_data_box_3) (delegate `CustomEvent_1`)))
    (:`then_7`
      (bind _asbp_personal_data_box_4 (cast `/Game/Level_Content/DataPrivacy/Blueprints/BP_PersonalDataBox` (`|GetArrayItem` (`self.StaticDataBoxes`) 7)))
      ;[1 1 1] Enable Physics again after being grabbed
      (add `/Game/VRTemplate/Blueprints/GrabComponent.OnGrabbed` (`/Game/Level_Content/DataPrivacy/Blueprints/BP_PersonalDataBox.GrabComponent` _asbp_personal_data_box_4) (delegate `CustomEvent_2`)))
    (:`then_8`
      (bind _asbp_personal_data_box_5 (cast `/Game/Level_Content/DataPrivacy/Blueprints/BP_PersonalDataBox` (`|GetArrayItem` (`self.StaticDataBoxes`) 8)))
      ;[1 1 1] Enable Physics again after being grabbed
      (add `/Game/VRTemplate/Blueprints/GrabComponent.OnGrabbed` (`/Game/Level_Content/DataPrivacy/Blueprints/BP_PersonalDataBox.GrabComponent` _asbp_personal_data_box_5) (delegate `CustomEvent_3`)))))

(event `OnGrabbed_Event`
  ;[1 1 1] Enable Physics again after being grabbed
  (set `/Game/Level_Content/DataPrivacy/Blueprints/BP_PersonalDataBox.IsHeld` true (stale `self.ReceiveTick` _asbp_personal_data_box))
  (set `/Game/VRTemplate/Blueprints/GrabComponent.bSimulateOnDrop` true (`/Game/Level_Content/DataPrivacy/Blueprints/BP_PersonalDataBox.GrabComponent` (stale `self.ReceiveTick` _asbp_personal_data_box)))
  (`PrimitiveComponent.SetEnableGravity` (`/Game/Level_Content/DataPrivacy/Blueprints/BP_PersonalDataBox.StaticMesh` (stale `self.ReceiveTick` _asbp_personal_data_box)) true))

(event `CustomEvent`
  ;[1 1 1] Enable Physics again after being grabbed
  (set `/Game/Level_Content/DataPrivacy/Blueprints/BP_PersonalDataBox.IsHeld` true (stale `self.ReceiveTick` _asbp_personal_data_box_2))
  (set `/Game/VRTemplate/Blueprints/GrabComponent.bSimulateOnDrop` true (`/Game/Level_Content/DataPrivacy/Blueprints/BP_PersonalDataBox.GrabComponent` (stale `self.ReceiveTick` _asbp_personal_data_box_2)))
  (`PrimitiveComponent.SetEnableGravity` (`/Game/Level_Content/DataPrivacy/Blueprints/BP_PersonalDataBox.StaticMesh` (stale `self.ReceiveTick` _asbp_personal_data_box_2)) true))

(event `CustomEvent_1`
  ;[1 1 1] Enable Physics again after being grabbed
  (set `/Game/Level_Content/DataPrivacy/Blueprints/BP_PersonalDataBox.IsHeld` true (stale `self.ReceiveTick` _asbp_personal_data_box_3))
  (set `/Game/VRTemplate/Blueprints/GrabComponent.bSimulateOnDrop` true (`/Game/Level_Content/DataPrivacy/Blueprints/BP_PersonalDataBox.GrabComponent` (stale `self.ReceiveTick` _asbp_personal_data_box_3)))
  (`PrimitiveComponent.SetEnableGravity` (`/Game/Level_Content/DataPrivacy/Blueprints/BP_PersonalDataBox.StaticMesh` (stale `self.ReceiveTick` _asbp_personal_data_box_3)) true))

(event `CustomEvent_2`
  ;[1 1 1] Enable Physics again after being grabbed
  (set `/Game/Level_Content/DataPrivacy/Blueprints/BP_PersonalDataBox.IsHeld` true (stale `self.ReceiveTick` _asbp_personal_data_box_4))
  (set `/Game/VRTemplate/Blueprints/GrabComponent.bSimulateOnDrop` true (`/Game/Level_Content/DataPrivacy/Blueprints/BP_PersonalDataBox.GrabComponent` (stale `self.ReceiveTick` _asbp_personal_data_box_4)))
  (`PrimitiveComponent.SetEnableGravity` (`/Game/Level_Content/DataPrivacy/Blueprints/BP_PersonalDataBox.StaticMesh` (stale `self.ReceiveTick` _asbp_personal_data_box_4)) true))

(event `CustomEvent_3`
  ;[1 1 1] Enable Physics again after being grabbed
  (set `/Game/Level_Content/DataPrivacy/Blueprints/BP_PersonalDataBox.IsHeld` true (stale `self.ReceiveTick` _asbp_personal_data_box_5))
  (set `/Game/VRTemplate/Blueprints/GrabComponent.bSimulateOnDrop` true (`/Game/Level_Content/DataPrivacy/Blueprints/BP_PersonalDataBox.GrabComponent` (stale `self.ReceiveTick` _asbp_personal_data_box_5)))
  (`PrimitiveComponent.SetEnableGravity` (`/Game/Level_Content/DataPrivacy/Blueprints/BP_PersonalDataBox.StaticMesh` (stale `self.ReceiveTick` _asbp_personal_data_box_5)) true))

(event `self.ReceiveBeginPlay`
  (bind _staticdataboxes (`self.StaticDataBoxes`))
  (bind _outactors (`GameplayStatics.GetAllActorsWithTag` "StaticDataBox"))
  (`KismetArrayLibrary.Array_Append` _staticdataboxes _outactors)
  (for _array_element _staticdataboxes
    (`self.SetActorHiddenInGame` _array_element true)))

(event `self.ReceiveActorBeginOverlap`
  (params (OtherActor :type "Actor Object Reference"))
  (bind _asbp_personal_data_box (cast `/Game/Level_Content/DataPrivacy/Blueprints/BP_PersonalDataBox` OtherActor)
    (:`then`
      (`/Game/Level_Content/DataPrivacy/Blueprints/BP_PersonalDataBox.TriggerTextOnNameBP` _asbp_personal_data_box)
      (`GameplayStatics.PlaySound2D` "/Game/Level_Content/DataPrivacy/Assets/Sounds/bubble-sound-43207.bubble-sound-43207" 1.0 1.0 0.0 null null)
      (`/Game/VRTemplate/Blueprints/GrabComponent.TryRelease` (`/Game/Level_Content/DataPrivacy/Blueprints/BP_PersonalDataBox.GrabComponent` _asbp_personal_data_box))
      (`PrimitiveComponent.SetCollisionResponseToChannel` (`/Game/Level_Content/DataPrivacy/Blueprints/BP_PersonalDataBox.StaticMesh` _asbp_personal_data_box) "ECC_PhysicsBody" "ECR_Ignore")
      (`self.K2_SetActorTransform` _asbp_personal_data_box (`/Game/Level_Content/DataPrivacy/Blueprints/BP_PersonalDataBox.InitialTransform` _asbp_personal_data_box) false false))
    (:`CastFailed`
      (bind _asbp_non_personal_data_box (cast `/Game/Level_Content/DataPrivacy/Blueprints/BP_NonPersonalDataBox` OtherActor))
      (`/Game/Level_Content/DataPrivacy/Blueprints/BP_NonPersonalDataBox.TriggerTextOnNameBP` _asbp_non_personal_data_box)
      (`GameplayStatics.PlaySound2D` "/Game/Level_Content/DataPrivacy/Assets/Sounds/bubble-sound-43207.bubble-sound-43207" 1.0 1.0 0.0 null null)
      (`/Game/VRTemplate/Blueprints/GrabComponent.TryRelease` (`/Game/Level_Content/DataPrivacy/Blueprints/BP_NonPersonalDataBox.GrabComponent` _asbp_non_personal_data_box))
      (`PrimitiveComponent.SetCollisionResponseToChannel` (`/Game/Level_Content/DataPrivacy/Blueprints/BP_NonPersonalDataBox.StaticMesh` _asbp_non_personal_data_box) "ECC_PhysicsBody" "ECR_Ignore")
      (`self.K2_SetActorTransform` _asbp_non_personal_data_box (`/Game/Level_Content/DataPrivacy/Blueprints/BP_NonPersonalDataBox.InitialTransform` _asbp_non_personal_data_box) false false))))

(fn `UserConstructionScript`)