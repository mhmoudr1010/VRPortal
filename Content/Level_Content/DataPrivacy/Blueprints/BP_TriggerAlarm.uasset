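; Data privacy level trigger that consumes data boxes on overlap and raises an alarm when one holds personal data.
; Both box types are marked finished; non-personal ones, and those typed "Personal", lose mesh, physics, collision and widgets.
; Personal data also plays BankAlarm, turns all small lamps red and runs a timeline, misleadingly named DirectionalLight, driving spot and point light intensity.
; When it finishes, lamps regain the material cached at BeginPlay.
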(event `self.ReceiveBeginPlay`
  (bind _outactors (`GameplayStatics.GetAllActorsOfClass` "/Game/Level_Content/DataPrivacy/Blueprints/Lamps/BP_SmallLamp.BP_SmallLamp_C"))
  (set `self.OriginalMaterial` (`PrimitiveComponent.GetMaterial` (`/Game/Level_Content/DataPrivacy/Blueprints/Lamps/BP_SmallLamp.StaticMesh` (`|GetArrayItem` _outactors)) 0)))

(event `self.ReceiveActorBeginOverlap`
  (params (OtherActor :type "Actor Object Reference"))
  (bind _billboard (`self.Billboard`))
  (bind _asbp_non_personal_data_box (cast `/Game/Level_Content/DataPrivacy/Blueprints/BP_NonPersonalDataBox` OtherActor)
    (:`then`
      (set `/Game/Level_Content/DataPrivacy/Blueprints/BP_NonPersonalDataBox.IsFinished` true _asbp_non_personal_data_box)
      (bind _staticmesh (`/Game/Level_Content/DataPrivacy/Blueprints/BP_NonPersonalDataBox.StaticMesh` _asbp_non_personal_data_box))
      (`SceneComponent.SetVisibility` _staticmesh false false)
      (`PrimitiveComponent.SetSimulatePhysics` _staticmesh false)
      (`PrimitiveComponent.SetCollisionEnabled` _staticmesh "NoCollision")
      (`|ExecutionSequence`
        (:`then_0`
          (`SceneComponent.SetVisibility` (`/Game/Level_Content/DataPrivacy/Blueprints/BP_NonPersonalDataBox.WidgetBack` _asbp_non_personal_data_box) false false)
          (bind _asbp_personal_data_box (cast `/Game/Level_Content/DataPrivacy/Blueprints/BP_PersonalDataBox` OtherActor :!label _label))
          (set `/Game/Level_Content/DataPrivacy/Blueprints/BP_PersonalDataBox.IsFinished` true _asbp_personal_data_box)
          (if (== (`/Game/Level_Content/DataPrivacy/Blueprints/BP_PersonalDataBox.DataType` _asbp_personal_data_box) "Personal")
            (bind _returnvalue (`GameplayStatics.SpawnSound2D` "/Game/Level_Content/DataPrivacy/Assets/Sounds/BankAlarm.BankAlarm" 1.0 1.0 0.0 null))
            (set `self.AudioComponent` _returnvalue)
            (bind _staticmesh_2 (`/Game/Level_Content/DataPrivacy/Blueprints/BP_PersonalDataBox.StaticMesh` _asbp_personal_data_box))
            (`SceneComponent.SetVisibility` _staticmesh_2 false false)
            (`PrimitiveComponent.SetSimulatePhysics` _staticmesh_2 false)
            (`PrimitiveComponent.SetCollisionEnabled` _staticmesh_2 "NoCollision")
            (`|ExecutionSequence`
              (:`then_0`
                (`SceneComponent.SetVisibility` (`/Game/Level_Content/DataPrivacy/Blueprints/BP_PersonalDataBox.WidgetForward` _asbp_personal_data_box) false false)
                ;[1 1 1] Change Lights to Red On Lamp1 and Lamp2
                (bind _outactors (`GameplayStatics.GetAllActorsOfClass` "/Game/Level_Content/DataPrivacy/Blueprints/Lamps/BP_SmallLamp.BP_SmallLamp_C"))
                (for _array_element _outactors
                  (`PrimitiveComponent.SetMaterial` (`/Game/Level_Content/DataPrivacy/Blueprints/Lamps/BP_SmallLamp.StaticMesh` _array_element) 0 "/Game/Level_Content/DataPrivacy/Assets/Bank_vault/materials/MI_RedAlarmMaterial.MI_RedAlarmMaterial")
                  (bind _outactors_2 (`GameplayStatics.GetAllActorsOfClass` "/Game/Level_Content/DataPrivacy/Blueprints/Lamps/BP_SmallLamp2.BP_SmallLamp2_C"))
                  (for _array_element_2 _outactors_2
                    (`PrimitiveComponent.SetMaterial` (`/Game/Level_Content/DataPrivacy/Blueprints/Lamps/BP_SmallLamp2.StaticMesh` _array_element_2) 0 "/Game/Level_Content/DataPrivacy/Assets/Bank_vault/materials/MI_RedAlarmMaterial.MI_RedAlarmMaterial")
                    (`SceneComponent.SetHiddenInGame` (`self.Billboard`) true true)
                    (bind (_direction _scalarintensity) (`Timeline|DirectionalLight` :!via `PlayFromStart`)
                      (:`Update`
                        (`LightComponent.SetIntensity` (`self.SpotLight`) _scalarintensity)
                        (`LightComponent.SetIntensity` (`self.SpotLight1`) _scalarintensity)
                        (`LightComponent.SetIntensity` (`self.SpotLight2`) _scalarintensity)
                        (`LightComponent.SetIntensity` (`self.SpotLight3`) _scalarintensity)
                        (`LightComponent.SetIntensity` (`self.SpotLight4`) _scalarintensity)
                        (`LightComponent.SetIntensity` (`self.SpotLight5`) _scalarintensity)
                        (`LightComponent.SetIntensity` (`self.PointLight5`) _scalarintensity)
                        (`LightComponent.SetIntensity` (`self.PointLight6`) _scalarintensity)
                        (`LightComponent.SetIntensity` (`self.PointLight7`) _scalarintensity)
                        (`LightComponent.SetIntensity` (`self.PointLight8`) _scalarintensity)
                        (`LightComponent.SetIntensity` (`self.PointLight9`) _scalarintensity)
                        (`LightComponent.SetIntensity` (`self.PointLight10`) _scalarintensity))
                      (:`Finished`
                        (for _array_element_3 _outactors
                          (`PrimitiveComponent.SetMaterial` (`/Game/Level_Content/DataPrivacy/Blueprints/Lamps/BP_SmallLamp.StaticMesh` _array_element_3) 0 (`self.OriginalMaterial`))
                          (for _array_element_4 _outactors_2
                            (`PrimitiveComponent.SetMaterial` (`/Game/Level_Content/DataPrivacy/Blueprints/Lamps/BP_SmallLamp2.StaticMesh` _array_element_4) 0 (`self.OriginalMaterial`))
                            (`SceneComponent.SetHiddenInGame` _billboard false true)
                            (`SceneComponent.SetHiddenInGame` _billboard true false))))))))
              (:`then_1`
                (`SceneComponent.SetVisibility` (`/Game/Level_Content/DataPrivacy/Blueprints/BP_PersonalDataBox.WidgetBack` _asbp_personal_data_box) false false))
              (:`then_2`
                (`SceneComponent.SetVisibility` (`/Game/Level_Content/DataPrivacy/Blueprints/BP_PersonalDataBox.WidgetRight` _asbp_personal_data_box) false false))
              (:`then_3`
                (`SceneComponent.SetVisibility` (`/Game/Level_Content/DataPrivacy/Blueprints/BP_PersonalDataBox.WidgetLeft` _asbp_personal_data_box) false false))
              (:`then_4`
                (`SceneComponent.SetVisibility` (`/Game/Level_Content/DataPrivacy/Blueprints/BP_PersonalDataBox.WidgetTop` _asbp_personal_data_box) false false))
              (:`then_5`
                (`SceneComponent.SetVisibility` (`/Game/Level_Content/DataPrivacy/Blueprints/BP_PersonalDataBox.WidgetBottom` _asbp_personal_data_box) false false)))))
        (:`then_1`
          (`SceneComponent.SetVisibility` (`/Game/Level_Content/DataPrivacy/Blueprints/BP_NonPersonalDataBox.WidgetBottom` _asbp_non_personal_data_box) false false))
        (:`then_2`
          (`SceneComponent.SetVisibility` (`/Game/Level_Content/DataPrivacy/Blueprints/BP_NonPersonalDataBox.WidgetForward` _asbp_non_personal_data_box) false false))
        (:`then_3`
          (`SceneComponent.SetVisibility` (`/Game/Level_Content/DataPrivacy/Blueprints/BP_NonPersonalDataBox.WidgetLeft` _asbp_non_personal_data_box) false false))
        (:`then_4`
          (`SceneComponent.SetVisibility` (`/Game/Level_Content/DataPrivacy/Blueprints/BP_NonPersonalDataBox.WidgetRight` _asbp_non_personal_data_box) false false))
        (:`then_5`
          (`SceneComponent.SetVisibility` (`/Game/Level_Content/DataPrivacy/Blueprints/BP_NonPersonalDataBox.WidgetTop` _asbp_non_personal_data_box) false false))))
    (:`CastFailed`
      (goto _label))))

(fn `UserConstructionScript`)