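; VR menu actor for HUB NPC interactions that hosts a Master_Widget and removes itself when the level-select panel fires its delete event.
; On BeginPlay it caches the VRPawn, or destroys itself without one, then enables input and adds a mapping context.
; Left and right menu-interact actions drive the pawn's WidgetInteraction components as simulated left mouse clicks.
; Camera-following rotation and mail-typing logic are present but disconnected.
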(event `self.ReceiveBeginPlay`
  (bind _returnvalue (`GameplayStatics.GetPlayerController` 0))
  (bind _asvrpawn (cast `/Game/VRTemplate/Blueprints/VRPawn` (`GameplayStatics.GetPlayerPawn` 0))
    (:`then`
      (bind _output_get (set `self.VRPawn` _asvrpawn))
      (`self.SetActorTickEnabled` _output_get true)
      (`self.EnableInput` _returnvalue)
      (`EnhancedInputSubsystemInterface.AddMappingContext` (pcsubsystem `EnhancedInputLocalPlayerSubsystem` _returnvalue) null 1 (struct))
      (bind _asmaster_widget (cast `/Game/Level_Content/DATAGOV/Widgets/DATAGOV/Master_Widget/Master_Widget` (`WidgetComponent.GetWidget` (`self.Widget`))))
      (add `/Game/Level_Content/DATAGOV/Widgets/DATAGOV/Level_Select/WB_Level_Select.Delete_Widget` (`/Game/Level_Content/DATAGOV/Widgets/DATAGOV/Master_Widget/Master_Widget.WB_Level_Select` _asmaster_widget) (delegate `Delete_Widget_Event`)))
    (:`CastFailed`
      (`self.K2_DestroyActor`))))

(event `typemail`)

(event `Delete_Widget_Event`
  (`self.K2_DestroyActor`))

(event `EnhancedInput|/Game/VRTemplate/Input/Actions/IA_Menu_Interact_Left`
  (params (ActionValue :type Boolean) (ElapsedSeconds :type "Float (double-precision)") (TriggeredSeconds :type "Float (double-precision)") (InputAction :type "InputAction Object Reference" :default "/Game/VRTemplate/Input/Actions/IA_Menu_Interact_Left.IA_Menu_Interact_Left"))
  (bind _widgetinteractionleft (`/Game/VRTemplate/Blueprints/VRPawn.WidgetInteractionLeft` (`self.VRPawn`)))
  (:`Started`
    (`WidgetInteractionComponent.PressPointerKey` _widgetinteractionleft "LeftMouseButton"))
  (:`Canceled`
    (`WidgetInteractionComponent.ReleasePointerKey` _widgetinteractionleft "LeftMouseButton" :!label _label))
  (:`Completed`
    (goto _label)))

(event `EnhancedInput|/Game/VRTemplate/Input/Actions/IA_Menu_Interact_Right`
  (params (ActionValue :type Boolean) (ElapsedSeconds :type "Float (double-precision)") (TriggeredSeconds :type "Float (double-precision)") (InputAction :type "InputAction Object Reference" :default "/Game/VRTemplate/Input/Actions/IA_Menu_Interact_Right.IA_Menu_Interact_Right"))
  (bind _widgetinteractionright (`/Game/VRTemplate/Blueprints/VRPawn.WidgetInteractionRight` (`self.VRPawn`)))
  (:`Started`
    (`WidgetInteractionComponent.PressPointerKey` _widgetinteractionright "LeftMouseButton"))
  (:`Canceled`
    (`WidgetInteractionComponent.ReleasePointerKey` _widgetinteractionright "LeftMouseButton" :!label _label_2))
  (:`Completed`
    (goto _label_2)))

(event `self.ReceiveTick`
  (params (DeltaSeconds :type "Float (single-precision)")))

(fn `Rotate_Menu`
  (params (`Delta Time` :type "Float (double-precision)"))
  (bind _defaultsceneroot (`self.DefaultSceneRoot`))
  (bind _transformcomponent (`PlayerCameraManager.TransformComponent` (`GameplayStatics.GetPlayerCameraManager` 0)))
  (bind (_returnvalue_roll _returnvalue_pitch _returnvalue_yaw) (`KismetMathLibrary.BreakRotator` (`KismetMathLibrary.RInterpTo` (`SceneComponent.K2_GetComponentRotation` _defaultsceneroot) (`SceneComponent.K2_GetComponentRotation` _transformcomponent) `Delta Time` 0.8)))
  (`self.K2_SetActorTransform` (`KismetMathLibrary.MakeTransform` (`KismetMathLibrary.VInterpTo` (`SceneComponent.K2_GetComponentLocation` _defaultsceneroot) (`SceneComponent.K2_GetComponentLocation` _transformcomponent) `Delta Time` 0.6) (`KismetMathLibrary.MakeRotator` 0.0 0.0 _returnvalue_yaw))))

(fn `UserConstructionScript`)