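; ScreenCin is the HUB cinema screen actor that plays a video chosen from the CinVideoMenu widget.
; On BeginPlay it takes the first CinVideoMenu widget it finds and binds to its Video1 and Exit dispatchers.
; Video1 opens a media source and swaps visibility between two planes to show the playback surface.
; Exit closes the media and swaps the planes back.
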(event `self.ReceiveBeginPlay`
  (bind _foundwidgets (`WidgetBlueprintLibrary.GetAllWidgetsOfClass` "/Game/Level_Content/HUB/Blueprints/CinemaNav/VideoSelect/CinVideoMenu.CinVideoMenu_C" false))
  (bind _output_get (set `self.Video Selector` (`|GetArrayItem` _foundwidgets)))
  (add `/Game/Level_Content/HUB/Blueprints/CinemaNav/VideoSelect/CinVideoMenu.Video 1` _output_get (delegate `Vid 1`))
  (add `/Game/Level_Content/HUB/Blueprints/CinemaNav/VideoSelect/CinVideoMenu.Exit` _output_get (delegate `Exit`)))

(event `Vid 1`
  (`MediaPlayer.OpenSource` (`self.Media`) "/Game/Level_Content/HUB/Blueprints/CinemaScreen/Vids/Test/WhatsApp_Video_2025-02-15_at_23_07_44_74df650b.WhatsApp_Video_2025-02-15_at_23_07_44_74df650b")
  (`self.VidStart`))

(event `Exit`
  (`MediaPlayer.Close` (`self.Media`))
  (`SceneComponent.SetHiddenInGame` (`self.Plane1`) false false)
  (`SceneComponent.SetHiddenInGame` (`self.Plane`) true false))

(event `VidStart`
  (`SceneComponent.SetHiddenInGame` (`self.Plane1`) true false)
  (`SceneComponent.SetHiddenInGame` (`self.Plane`) false false))

(fn `UserConstructionScript`)