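; SnapTPZone is a VR teleport zone in the HUB that snaps the player to its origin.
; When the teleport visualizer overlaps Box, the zone shows its Niagara effect and hides the visualizer's ring and play-area bounds.
; End overlap hides the effect, but the code to unhide those visuals is disconnected.
; A VR pawn entering Box1 has its VR origin moved to the zone root, adopting its rotation if Directional.
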(event `self.Box.OnComponentBeginOverlap`
  (params (OverlappedComponent :type "PrimitiveComponent Object Reference") (OtherActor :type "Actor Object Reference") (OtherComp :type "PrimitiveComponent Object Reference") (OtherBodyIndex :type Integer) (bFromSweep :type Boolean) (SweepResult :type "HitResult Structure (by ref)"))
  (cast `/Game/VRTemplate/Blueprints/VRTeleportVisualizer` OtherActor)
  (`SceneComponent.SetHiddenInGame` (`self.Niagara`) false false)
  (bind _outactors (`GameplayStatics.GetAllActorsOfClass` "/Game/VRTemplate/Blueprints/VRTeleportVisualizer.VRTeleportVisualizer_C"))
  (`SceneComponent.SetHiddenInGame` (`/Game/VRTemplate/Blueprints/VRTeleportVisualizer.NS_TeleportRing` (`|GetArrayItem` _outactors)) true false)
  (`SceneComponent.SetHiddenInGame` (`/Game/VRTemplate/Blueprints/VRTeleportVisualizer.NS_PlayAreaBounds` (`|GetArrayItem` _outactors)) true false))

(event `self.Box.OnComponentEndOverlap`
  (params (OverlappedComponent :type "PrimitiveComponent Object Reference") (OtherActor :type "Actor Object Reference") (OtherComp :type "PrimitiveComponent Object Reference") (OtherBodyIndex :type Integer))
  (`SceneComponent.SetHiddenInGame` (`self.Niagara`) true false)
  (bind _outactors (`GameplayStatics.GetAllActorsOfClass` "/Game/VRTemplate/Blueprints/VRTeleportVisualizer.VRTeleportVisualizer_C")))

(event `self.Box1.OnComponentBeginOverlap`
  (params (OverlappedComponent :type "PrimitiveComponent Object Reference") (OtherActor :type "Actor Object Reference") (OtherComp :type "PrimitiveComponent Object Reference") (OtherBodyIndex :type Integer) (bFromSweep :type Boolean) (SweepResult :type "HitResult Structure (by ref)"))
  (bind (_returnvalue_location _returnvalue_rotation) (`KismetMathLibrary.BreakTransform` (`SceneComponent.K2_GetComponentToWorld` (`self.DefaultSceneRoot`))))
  (bind _asvrpawn (cast `/Game/VRTemplate/Blueprints/VRPawn` OtherActor))
  (if (`self.Directional?`)
    (bind _vrorigin (`/Game/VRTemplate/Blueprints/VRPawn.VROrigin` _asvrpawn))
    (`SceneComponent.K2_SetWorldLocationAndRotation` _vrorigin _returnvalue_location _returnvalue_rotation false true)
    (else
      (`SceneComponent.K2_SetWorldLocationAndRotation` _vrorigin _returnvalue_location (`SceneComponent.K2_GetComponentRotation` _vrorigin) false true))))

(fn `UserConstructionScript`)