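; Grabbable VR trophy prop for the hub that makes metal sounds and returns to its pillar after being let go.
; Grabbing plays a random sound and shows a plane; dropping hides it and, after two seconds without a regrab, teleports the mesh to its stored pillar transform.
; Non-pawn hits play speed-dependent impact sounds, throttled by a DoOnce with delayed reset.
; MoveCheck and Tick are empty, and the camera-facing logic is disconnected.
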(event `self.S_Paper_Towel_Roll_vjxodjps_lod5_Var1.OnComponentHit`
  (params (HitComponent :type "PrimitiveComponent Object Reference") (OtherActor :type "Actor Object Reference") (OtherComp :type "PrimitiveComponent Object Reference") (NormalImpulse :type "Vector Structure") (Hit :type "HitResult Structure (by ref)"))
  (bind _returnvalue (`KismetMathLibrary.VSize` (`SceneComponent.GetComponentVelocity` HitComponent)))
  (bind _returnvalue_2 (- (`KismetMathLibrary.FMin` (/ _returnvalue 100.0) 1.0) 0.5))
  (cast `/Game/VRTemplate/Blueprints/VRPawn` OtherActor
    (:`CastFailed`
      (`self.MoveCheck`)
      (`|ExecutionSequence`
        (:`then_0`
          (`/Engine/EditorBlueprintResources/StandardMacros.DoOnce` false :!label _label
            (:`Completed`
              (if (> _returnvalue 40.0)
                (if (not (> _returnvalue 140.0))
                  (switch `int` (`KismetMathLibrary.RandomIntegerInRange` 0 3)
                    (:`0`
                      (`GameplayStatics.SpawnSoundAttached` "/Game/Level_Content/DATAGOV/SoundFX/General/Mubkhara/heavy_metal_item_imp__1___mp3cut_net_.heavy_metal_item_imp__1___mp3cut_net_" (`self.S_Paper_Towel_Roll_vjxodjps_lod5_Var1`) "None" (0.0 0.0 0.0) (struct) "KeepRelativeOffset" false _returnvalue_2 1.0 0.0 "/Game/Level_Content/DATAGOV/SoundFX/ImpactSoundAttenuation.ImpactSoundAttenuation" null))
                    (:`1`
                      (`GameplayStatics.SpawnSoundAttached` "/Game/Level_Content/DATAGOV/SoundFX/General/Mubkhara/heavy_metal_item_imp__2___mp3cut_net_.heavy_metal_item_imp__2___mp3cut_net_" (`self.S_Paper_Towel_Roll_vjxodjps_lod5_Var1`) "None" (0.0 0.0 0.0) (struct) "KeepRelativeOffset" false _returnvalue_2 1.0 0.0 "/Game/Level_Content/DATAGOV/SoundFX/ImpactSoundAttenuation.ImpactSoundAttenuation" null))
                    (:`2`
                      (`GameplayStatics.SpawnSoundAttached` "/Game/Level_Content/DATAGOV/SoundFX/General/Mubkhara/heavy_metal_item_imp__4___mp3cut_net_.heavy_metal_item_imp__4___mp3cut_net_" (`self.S_Paper_Towel_Roll_vjxodjps_lod5_Var1`) "None" (0.0 0.0 0.0) (struct) "KeepRelativeOffset" false _returnvalue_2 1.0 0.0 "/Game/Level_Content/DATAGOV/SoundFX/ImpactSoundAttenuation.ImpactSoundAttenuation" null))
                    (:`3`
                      (`GameplayStatics.SpawnSoundAttached` "/Game/Level_Content/DATAGOV/SoundFX/General/Mubkhara/heavy_metal_item_imp__mp3cut_net_.heavy_metal_item_imp__mp3cut_net_" (`self.S_Paper_Towel_Roll_vjxodjps_lod5_Var1`) "None" (0.0 0.0 0.0) (struct) "KeepRelativeOffset" false 1.0 1.0 0.0 "/Game/Level_Content/DATAGOV/SoundFX/ImpactSoundAttenuation.ImpactSoundAttenuation" null)))
                  (else
                    (`GameplayStatics.SpawnSoundAttached` "/Game/Level_Content/DATAGOV/SoundFX/General/Mubkhara/heavy_metal_item_imp__3___mp3cut_net_.heavy_metal_item_imp__3___mp3cut_net_" (`self.S_Paper_Towel_Roll_vjxodjps_lod5_Var1`) "None" (0.0 0.0 0.0) (struct) "KeepRelativeOffset" false _returnvalue_2 1.0 0.0 "/Game/Level_Content/DATAGOV/SoundFX/ImpactSoundAttenuation.ImpactSoundAttenuation" null)))))))
        (:`then_1`
          (`KismetSystemLibrary.Delay` 0.2)
          (goto _label :!via `Reset`))))))

(event `self.GrabComponent.OnGrabbed`
  (params (`Motion Controller` :type "MotionControllerComponent Object Reference"))
  (set `self.Grabbed?` true)
  (`SceneComponent.SetHiddenInGame` (`self.Plane`) false true)
  (switch `int` (`KismetMathLibrary.RandomIntegerInRange` 0 2)
    (:`0`
      (`GameplayStatics.SpawnSoundAttached` "/Game/Level_Content/DATAGOV/SoundFX/General/MetalBowl/small_light_Metal_Bowl_grab.small_light_Metal_Bowl_grab" (`self.S_Paper_Towel_Roll_vjxodjps_lod5_Var1`) "None" (0.0 0.0 0.0) (struct) "KeepRelativeOffset" false 0.5 1.0 0.0 "/Game/Level_Content/DATAGOV/SoundFX/ImpactSoundAttenuation.ImpactSoundAttenuation" null))
    (:`1`
      (`GameplayStatics.SpawnSoundAttached` "/Game/Level_Content/DATAGOV/SoundFX/General/MetalBowl/small_light_Metal_Bowl_grab__1_.small_light_Metal_Bowl_grab__1_" (`self.S_Paper_Towel_Roll_vjxodjps_lod5_Var1`) "None" (0.0 0.0 0.0) (struct) "KeepRelativeOffset" false 0.5 1.0 0.0 "/Game/Level_Content/DATAGOV/SoundFX/ImpactSoundAttenuation.ImpactSoundAttenuation" null))
    (:`2`
      (`GameplayStatics.SpawnSoundAttached` "/Game/Level_Content/DATAGOV/SoundFX/General/MetalBowl/small_light_Metal_Bowl_grab__2_.small_light_Metal_Bowl_grab__2_" (`self.S_Paper_Towel_Roll_vjxodjps_lod5_Var1`) "None" (0.0 0.0 0.0) (struct) "KeepRelativeOffset" false 0.5 1.0 0.0 "/Game/Level_Content/DATAGOV/SoundFX/ImpactSoundAttenuation.ImpactSoundAttenuation" null))))

(event `self.GrabComponent.OnDropped`
  (set `self.Grabbed?` false)
  (`SceneComponent.SetHiddenInGame` (`self.Plane`) true true)
  (`KismetSystemLibrary.Delay` 2.0)
  (if (not (`self.Grabbed?`))
    (`SceneComponent.K2_SetWorldLocationAndRotation` (`self.S_Paper_Towel_Roll_vjxodjps_lod5_Var1`) (`self.PillarLoc`) (`self.PillarRot`) false true)
    (`PrimitiveComponent.SetAllPhysicsLinearVelocity` (`self.S_Paper_Towel_Roll_vjxodjps_lod5_Var1`) (0.0 0.0 0.0) false)))

(event `MoveCheck`)

(event `self.ReceiveTick`
  (params (DeltaSeconds :type "Float (single-precision)")))

(fn `UserConstructionScript`)