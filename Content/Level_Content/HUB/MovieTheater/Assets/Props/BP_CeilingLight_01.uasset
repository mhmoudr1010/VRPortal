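; Recessed ceiling light prop for the HUB movie theater, with a Lit switch and configurable lighting.
; The construction script applies intensity, indirect intensity, radius, color temperature and spot cone angles to its light components and swaps the fixture mesh to a lit material.
; When unlit, it zeroes the lights' attenuation radius instead of hiding them and applies the standard fixture material.
; The event graph is empty.
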(fn `UserConstructionScript`
  (bind _ceilinglightsunk_01 (`self.CeilingLightSunk_01`))
  (bind _spotlight (`self.SpotLight`))
  (bind _array (`|MakeArray` _spotlight null null null :!type "PointLightComponent Object Reference"))
  (if (`self.Lit`)
    (for _array_element _array
      (`LightComponent.SetIndirectLightingIntensity` _array_element (`self.Indirect Intensity`))
      (`SpotLightComponent.SetInnerConeAngle` _spotlight (`self.Inner Cone Range`))
      (`SpotLightComponent.SetOuterConeAngle` _spotlight (`self.Outer Cone Range`))
      (`LocalLightComponent.SetAttenuationRadius` _array_element (`self.Radius`))
      (`LightComponent.SetIntensity` _array_element (`self.Intensity`))
      (`LightComponent.SetTemperature` _array (`self.Temperature`))
      (`PrimitiveComponent.SetMaterial` _ceilinglightsunk_01 0 "/Game/Level_Content/HUB/MovieTheater/Assets/Props/Materials/MI_Lit.MI_Lit"))
    (else
      (for _array_element_2 _array
        (`LocalLightComponent.SetAttenuationRadius` _array_element_2 0.0)
        (`LocalLightComponent.SetAttenuationRadius` _array_element_2 0.0)
        (`PrimitiveComponent.SetMaterial` _ceilinglightsunk_01 0 "/Game/Level_Content/HUB/MovieTheater/Assets/Props/Materials/MI_CeilingLight_01.MI_CeilingLight_01")))))